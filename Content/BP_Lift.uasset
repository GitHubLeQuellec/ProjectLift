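; BP_Lift is a procedurally built multi-level lift, with a shaft and a car placed at a random level.
; The construction script stacks four meshes per level, one mirrored, using NbLevels and Height.
; It stores the car as Liftref and snaps two meshes to it, one mirrored via negative X scale.
; Tick runs constant interpolation on the car's Z, but only Current and InterpSpeed (fed DeltaSeconds) are set.
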(event EventBeginPlay)

(event Collision|EventActorBeginOverlap
  (params (OtherActor :type Actor%20Object%20Reference)))

(event EventTick
  (params (DeltaSeconds :type Float%20%28single-precision%29))
  (bind _liftref (Variables|Default|GetLiftref))
  (Transformation|SetRelativeLocation _liftref (Math|Vector|MakeVector 0.0 0.0 (Math|Interpolation|FInterptoConstant (.z (Variables|/Script/Engine.SceneComponent|GetRelativeLocation _liftref)) 0.0 0.0 DeltaSeconds)) false false))

(fn ConstructionScript
  (bind _nblevels (Variables|Default|GetNbLevels))
  (bind _height (Variables|Default|GetHeight))
  (bind _returnvalue (Math|Random|RandomInteger _nblevels))
  (bind _returnvalue_2 (* _returnvalue _height))
  (for _index (range 0 (- (Variables|Default|GetNbLevels) 1))
    (AddComponent|AddStaticMeshComponent false (Math|Transform|MakeTransform (Math|Vector|MakeVector 0.0 0.0 (* _index (Variables|Default|GetHeight))) "0, 0, 0" "1.000000,1.000000,1.000000"))
    (AddComponent|AddStaticMeshComponent false (Math|Transform|MakeTransform (Math|Vector|MakeVector 0.0 0.0 (* _index (Variables|Default|GetHeight))) "0, 0, 0" "1.000000,1.000000,1.000000"))
    (AddComponent|AddStaticMeshComponent false (Math|Transform|MakeTransform (Math|Vector|MakeVector 0.0 0.0 (* _index (Variables|Default|GetHeight))) "0, 0, 0" "1.000000,1.000000,1.000000"))
    (AddComponent|AddStaticMeshComponent false (Math|Transform|MakeTransform (Math|Vector|MakeVector 0.0 0.0 (* _index (Variables|Default|GetHeight))) "0, 0, 0" "-1.000000,1.000000,1.000000")))
  (bind _returnvalue_3 (AddComponent|AddStaticMeshComponent false (Math|Transform|MakeTransform (Math|Vector|MakeVector 0.0 0.0 _returnvalue_2) "0, 0, 0" "1.000000,1.000000,1.000000")))
  (Variables|Default|SetLiftref _returnvalue_3)
  (bind _returnvalue_4 (AddComponent|AddStaticMeshComponent false (Math|Transform|MakeTransform (Math|Vector|MakeVector 0.0 0.0 _returnvalue_2) "0, 0, 0" "1.000000,1.000000,1.000000")))
  (Transformation|AttachComponentToComponent _returnvalue_4 (Variables|Default|GetLiftref) "None" "SnapToTarget" "SnapToTarget" "SnapToTarget" true)
  (bind _returnvalue_5 (AddComponent|AddStaticMeshComponent false (Math|Transform|MakeTransform (Math|Vector|MakeVector 0.0 0.0 _returnvalue_2) "0, 0, 0" "-1.000000,1.000000,1.000000")))
  (Transformation|AttachComponentToComponent _returnvalue_5 (Variables|Default|GetLiftref) "None" "SnapToTarget" "SnapToTarget" "KeepWorld" true))